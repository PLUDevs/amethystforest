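; Buoy actor that floats on the ocean waves supplied by an OceanManager.
; Every tick it loops over its WaterTestPoints and runs ProcessWaveHeightAtPoint on each, passing the Buoy component, actor transform, ocean manager and game time.
; The component's mass is split evenly across the points, so buoyancy is evaluated per point rather than for the body as a whole.
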(event `self.ReceiveTick`
  (params (DeltaSeconds :type "Float (single-precision)"))
  (bind _watertestpoints (`self.WaterTestPoints`))
  (bind _buoy (`self.Buoy`))
  ;[1 1 1] When Game Starts (tick event)
  ;[1 0.3877 0] For each test point in array
  (for _array_element _watertestpoints
    ;[1 0.04544 0] Process Wave Height at Point
    (`/Game/Blueprints/OceanManager/OceanManagerHelper.ProcessWaveHeightAtPoint` _array_element _buoy (`self.OceanManager`) (`self.GetTransform`) (/ (`PrimitiveComponent.GetMass` _buoy) (`KismetMathLibrary.Conv_IntToDouble` (`KismetArrayLibrary.Array_Length` _watertestpoints))) 10.0 1.0 (`KismetSystemLibrary.GetGameTimeInSeconds`))))

(fn `UserConstructionScript`)