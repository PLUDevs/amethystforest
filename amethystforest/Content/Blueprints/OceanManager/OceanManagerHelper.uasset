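; Ocean helper functions that apply point-based buoyancy to a primitive component using the OceanManager's wave height.
; EvalWaveHeightAtPoint transforms the point by the actor transform and compares it to the wave, cubing the thickness-normalized offset into a clamped strength.
; ProcessWaveHeightAtPoint uses that strength and point mass to push up by displacement ratio when submerged, or down at gravity scale otherwise.
; The force is applied at the untransformed input location.
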(fn `EvalWaveHeightAtPoint`
  (params (`Point Location` :type "Object.Vector Structure") (`Actor Transform` :type "Object.Transform Structure") (`Ocean Manager` :type "OceanManager Object Reference") (`Point Thickness` :type "Float (double-precision)") (Time :type "Float (double-precision)"))
  (returns (`Is Under` :type Boolean) (Amount :type "Float (double-precision)") (Delta :type "Float (double-precision)") (`Wave Intersect Point` :type "Object.Vector Structure") (`Wave Height` :type "Float (double-precision)"))
  (bind _returnvalue (`KismetMathLibrary.TransformLocation` `Actor Transform` `Point Location`))
  (bind _z (.z _returnvalue))
  (bind _returnvalue_2 (`OceanManager.GetWaveHeightValue` `Ocean Manager` _returnvalue Time))
  (bind _z_2 (.z _returnvalue_2))
  (bind _returnvalue_3 (- _z_2 _z))
  (return (> _returnvalue_3 0.0) (`KismetMathLibrary.Abs` (`KismetMathLibrary.FClamp` (`KismetMathLibrary.MultiplyMultiply_FloatFloat` (/ _returnvalue_3 `Point Thickness`) 3.0) -1.0 1.0)) _returnvalue_3 (`KismetMathLibrary.MakeVector` (.x (+ _returnvalue_2 _returnvalue)) (.y (+ _returnvalue_2 _returnvalue)) _z) _z_2))

(fn `ProcessWaveHeightAtPoint`
  (params (`Point Location` :type "Object.Vector Structure") (`Primitive Component` :type "PrimitiveComponent Object Reference") (`Ocean Manager` :type "OceanManager Object Reference") (`Actor Transform` :type "Object.Transform Structure") (`Mass Of Point` :type "Float (double-precision)") (`Point Thickness` :type "Float (double-precision)") (`Displacement Ratio` :type "Float (double-precision)") (Time :type "Float (double-precision)"))
  (returns (IsUnder :type Boolean))
  (bind (_is_under _amount) (`self.EvalWaveHeightAtPoint` `Point Location` `Actor Transform` `Ocean Manager` `Point Thickness` Time))
  (if _is_under
    (`PrimitiveComponent.AddForceAtLocation` `Primitive Component` (* (* (`KismetMathLibrary.MakeVector` 0.0 0.0 (* `Displacement Ratio` 980.0)) `Mass Of Point`) _amount) `Point Location` "None")
    (else
      (`PrimitiveComponent.AddForceAtLocation` `Primitive Component` (* (* (`KismetMathLibrary.MakeVector` 0.0 0.0 -980.0) `Mass Of Point`) _amount) `Point Location` "None")))
  (return _is_under))